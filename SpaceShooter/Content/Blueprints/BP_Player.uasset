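; Player Blueprint that plays a spinning spawn animation and moves on the X/Z plane from axis input.
; BeginPlay caches BP_GameMode, then a timeline lerps location by a Distance offset while spinning yaw, setting MovedEnabled when finished.
; MoveUp and MoveRight set speeds that Tick applies as a swept offset each frame, without delta-time scaling or checking MovedEnabled.
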(event EventBeginPlay
  ;[1 1 1] Player Spawn Animation
  (bind _asbp_game_mode (Utilities|Casting|CastToBP_GameMode (Game|GetGameMode)))
  (Variables|Default|SetBP_GameMode _asbp_game_mode)
  (Variables|Default|SetYaw (.Yaw (Math|Rotator|BreakRotator (Transformation|GetActorRotation))))
  (Variables|Default|SetSpawnLocation (Transformation|GetActorLocation))
  (bind _speed (Timeline|SpawnAnimation Play)
    (:Update
      (Transformation|SetActorLocation (Math|Vector|Lerp(Vector) (Variables|Default|GetSpawnLocation) (+ (Variables|Default|GetSpawnLocation) (Variables|Default|GetDistance)) _speed) false false)
      (Transformation|SetActorRotation (Math|Rotator|Lerp(Rotator) "0, 0, 0" (Math|Rotator|MakeRotator 0.0 0.0 (+ (Variables|Default|GetYaw) (Variables|Default|GetSpawnSpinCount))) _speed)))
    (:Finished
      (Variables|Default|SetMovedEnabled true))))

(event EventTick
  (params (DeltaSeconds :type Float%20%28single-precision%29))
  (Variables|Default|SetDeltaSeconds DeltaSeconds)
  (Transformation|SetActorLocation (+ (Transformation|GetActorLocation) (Math|Vector|MakeVector (Variables|Default|GetHozSpeed) 0.0 (Variables|Default|GetVertSpeed))) true false))

(event Input|AxisEvents|InputAxisMoveUp
  (params (AxisValue :type Float%20%28single-precision%29))
  (Variables|Default|SetVertSpeed (* (Variables|Default|GetMovementsSpeed) AxisValue)))

(event Input|AxisEvents|InputAxisMoveRight
  (params (AxisValue :type Float%20%28single-precision%29))
  (Variables|Default|SetHozSpeed (* (Variables|Default|GetMovementsSpeed) AxisValue)))

(fn ConstructionScript)